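; BP_GameManager is a manager Blueprint that holds references to an object factory and a pool and relays player death.
; Init events store the factory and pool references; UseFactory asks the factory to spawn an object of a given type at a transform.
; GetPool returns the stored pool, and PlayerDieCall fires the OnPlayerDie dispatcher.
; UsePoolGm and BindearEvento are empty stubs, and the dispatcher's bind node is never executed.
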(event `/Game/Scripts/BPI_InitGM.InitFactory`
  (params (Factory :type "/Game/Scripts/BP_Factory Object Reference"))
  (set `self.Factory` Factory))

(event `/Game/Scripts/BPI_GM.UseFactory`
  (params (Type :type "/Game/Scripts/EProjectyleType Enum" :default "NewEnumerator0") (originPosition :type "Transform Structure"))
  (`/Game/Scripts/BP_Factory.SpawnObject` (`self.Factory`) originPosition Type))

(event `/Game/Scripts/BPI_InitGM.InitPoolSize`
  (params (PoolObject :type "/Game/Scripts/BP_PoolManager Object Reference"))
  (bind _output_get (set `self.PoolSize` PoolObject))
  (`KismetSystemLibrary.PrintString` (`KismetStringLibrary.Concat_StrStr` "Inicializacion de pool hecha" (`KismetSystemLibrary.GetDisplayName` _output_get))))

(event `/Game/Scripts/BPI_GM.UsePoolGm`)

(event `/Game/Scripts/BPI_GM.PlayerDieCall`
  (`self.onPlayerDie`))

(fn `BindearEvento`
  (params (NewParam :type "Object Object Reference"))
  (return))

(fn `GetPool`
  (returns (poolrefe :type "/Game/Scripts/BP_PoolManager Object Reference"))
  (return (`self.PoolSize`)))