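; Base projectile actor that flies in a straight line toward where the player pawn was when it was initialized.
; INIT caches direction, faces the player and sets a lifetime timer on DestroySelf, whose DestroyActor call is disconnected; Tick applies swept movement.
; Move supports pool-style reuse by disabling the actor, teleporting it to a given transform, re-enabling it and rerunning INIT.
; The Parry event is an empty stub.
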(event `self.ReceiveBeginPlay`
  (`self.INIT`))

(event `self.ReceiveTick`
  (params (DeltaSeconds :type "Float (single-precision)"))
  (`self.K2_AddActorWorldOffset` (* (* (`self.Speed`) (`self.Direction`)) DeltaSeconds) true))

(event `/Game/Scripts/BPI_PARRY.Parry`)

(fn `ActivarObjeto`
  (`self.SetActorHiddenInGame` false)
  (`self.SetActorEnableCollision` true)
  (`self.SetActorTickEnabled` true))

(fn `DesactivarObjeto`
  (`self.SetActorHiddenInGame` true)
  (`self.SetActorEnableCollision` false)
  (`self.SetActorTickEnabled` false))

(fn `DestroySelf`)

(fn `INIT`
  (bind _returnvalue (`self.K2_GetActorLocation`))
  (bind _returnvalue_2 (`self.K2_GetActorLocation` (`self.PlayerRef`)))
  (set `self.PlayerRef` (`GameplayStatics.GetPlayerPawn` 0))
  (set `self.Direction` (`KismetMathLibrary.Normal` (- _returnvalue_2 _returnvalue)))
  (`self.K2_SetActorRotation` (`KismetMathLibrary.FindLookAtRotation` _returnvalue _returnvalue_2))
  (`KismetSystemLibrary.K2_SetTimer` null "DestroySelf" (`self.LifeTime`)))

(fn `Move`
  (params (t :type "Transform Structure"))
  (returns (objectref :type "Object Object Reference"))
  (`KismetSystemLibrary.PrintString` (`KismetStringLibrary.Concat_StrStr` "Objeto   " (`KismetSystemLibrary.GetDisplayName` self) " Movido a" (`KismetStringLibrary.Conv_TransformToString` t)))
  (`self.DesactivarObjeto`)
  (`self.K2_SetActorTransform` self t false false)
  (`self.ActivarObjeto`)
  (`self.INIT`)
  (return self))

(fn `UserConstructionScript`)