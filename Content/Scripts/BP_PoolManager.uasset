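; BP_PoolManager is an object pool that holds references to pooled objects and hands them out at random.
; On BeginPlay it passes itself to the Game Instance through InitPoolSizeMessage and exposes its PoolSize via GetPoolSize.
; AddObject stores objects uniquely, while UsePool removes and returns a random entry without checking for an empty pool.
; Both operations print debug messages with the object's name.
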(event `self.ReceiveBeginPlay`
  (message `/Game/Scripts/BPI_InitGM.InitPoolSize` (`GameplayStatics.GetGameInstance`) self))

(event `/Game/Scripts/BPI_Pool.AddObject`
  (params (referenceObject :type "Object Object Reference (by ref)"))
  (`KismetSystemLibrary.PrintString` (`KismetStringLibrary.Concat_StrStr` "Objetoi Añadido  " (`KismetSystemLibrary.GetDisplayName` referenceObject)))
  (`KismetArrayLibrary.Array_AddUnique` (`self.PoolObjects`) referenceObject))

(fn `GetPoolSize`
  (returns (PoolSize :type Integer))
  (return (`self.PoolSize`)))

(fn `UsePool`
  (returns (ReturnReference :type "Object Object Reference"))
  (bind _lastobject (`self.LastObject`))
  (bind _output_get (set `self.LastObject` (`|GetArrayItem` (`self.PoolObjects`) (`KismetMathLibrary.RandomIntegerInRange` 0 (- (`KismetArrayLibrary.Array_Length` (`self.PoolObjects`)) 1)))))
  (`KismetArrayLibrary.Array_RemoveItem` (`self.PoolObjects`) _output_get)
  (`KismetSystemLibrary.PrintString` (`KismetStringLibrary.Concat_StrStr` "Objetoi RETORNADO" (`KismetSystemLibrary.GetDisplayName` _lastobject)))
  (return _lastobject))

(fn `UserConstructionScript`)