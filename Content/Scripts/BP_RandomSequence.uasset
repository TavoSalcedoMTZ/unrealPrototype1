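; Randomized spawner that spawns objects at the transforms of actors tagged PositionGroups, gathered at BeginPlay.
; A self-rescheduling delay loop picks a random position each cycle, with a jittered interval scaled by an acceleration factor.
; Early spawns request a random type from the GameInstance factory.
; Past a count limit, it takes objects from the GameInstance's pool and moves those implementing BPI_PARRY to the chosen position.
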(event `self.ReceiveBeginPlay`
  (`KismetArrayLibrary.Array_Clear` (`self.PositionActors`))
  (bind _outactors (`GameplayStatics.GetAllActorsWithTag` "PositionGroups"))
  (for _array_element _outactors
    (`KismetArrayLibrary.Array_AddUnique` (`self.PositionActors`) (`self.GetTransform` _array_element))
    (`KismetSystemLibrary.Delay` 0.2)
    (`self.StartSpawnLoop`)))

(event `ExecuteSpawn`
  (set `self.BaseInterval` (* (`self.BaseInterval`) (`self.AcelartionFactor`)))
  (bind _output_get (set `self.RandomIndex` (`KismetMathLibrary.RandomIntegerInRange` 0 (- (`KismetArrayLibrary.Array_Length` (`self.PositionActors`)) 1))))
  (if (<= (`self.SpawnCount`) 30)
    (bind _output (`|GetArrayItem` (`self.PositionActors`) _output_get))
    (message `/Game/Scripts/BPI_GM.UseFactory` (`GameplayStatics.GetGameInstance`) (`BlueprintSetLibrary.Set_GetItemByIndex` (`self.EnumTypes`) (`KismetMathLibrary.RandomIntegerInRange` 0 (- (`BlueprintSetLibrary.Set_Length` (`self.EnumTypes`)) 1))) _output)
    (`KismetSystemLibrary.PrintString` "Ciclo terminado")
    (`self.Sum`)
    (`self.StartSpawnLoop`)
    (else
      (`KismetSystemLibrary.PrintString` "Limite alcanzado usa pools")
      (bind _poolrefe (`self.PoolRefGet`))
      (bind _returnreference (message `/Game/Scripts/BPI_Pool.UsePool` _poolrefe))
      (if (`KismetSystemLibrary.DoesImplementInterface` _returnreference "/Game/Scripts/BPI_PARRY.BPI_PARRY_C")
        (message `/Game/Scripts/BPI_PARRY.Move` _returnreference _output)
        (`self.StartSpawnLoop`)
        (else
          (`KismetSystemLibrary.PrintString` "No contiene interfaz")
          (`self.StartSpawnLoop`))))))

(event `StartSpawnLoop`
  (`KismetSystemLibrary.Delay` (`KismetMathLibrary.RandomFloatInRange` (- (`self.BaseInterval`) (`self.RandomVariation`)) (+ (`self.BaseInterval`) (`self.RandomVariation`))))
  (`self.ExecuteSpawn`))

(fn `PoolRefGet`
  (returns (poolrefe :type "/Game/Scripts/BP_PoolManager Object Reference"))
  (bind _poolrefe (message `/Game/Scripts/BPI_GM.GetPool` (`GameplayStatics.GetGameInstance`)))
  (return _poolrefe))

(fn `Sum`
  (set `self.SpawnCount` (+ (`self.SpawnCount`) 1)))

(fn `UserConstructionScript`)