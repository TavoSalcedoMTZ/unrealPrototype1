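; BP_FollowTarget is an actor that chases the first player's pawn.
; Each tick it rotates to face the pawn and moves along the normalized direction toward it, scaled by Speed and delta time.
; Movement uses a swept world offset, while the rotation snaps straight to the look-at angle without interpolation.
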(event `self.ReceiveTick`
  (params (DeltaSeconds :type "Float (single-precision)"))
  (bind _returnvalue (`self.K2_GetActorLocation`))
  (bind _returnvalue_2 (`self.K2_GetActorLocation` (`self.PlayerRef`)))
  (set `self.PlayerRef` (`GameplayStatics.GetPlayerPawn` 0))
  (bind _output_get (set `self.Direction` (`KismetMathLibrary.Normal` (- _returnvalue_2 _returnvalue))))
  (`self.K2_SetActorRotation` (`KismetMathLibrary.FindLookAtRotation` _returnvalue _returnvalue_2))
  (`self.K2_AddActorWorldOffset` (* (* (`self.Speed`) _output_get) DeltaSeconds) true))

(fn `UserConstructionScript`
  (`parent.UserConstructionScript`))