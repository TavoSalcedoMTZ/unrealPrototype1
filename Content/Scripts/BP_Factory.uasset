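; Factory Blueprint that spawns objects by type and hands them to an object pool.
; On BeginPlay it registers itself with the Game Instance and prints a debug string.
; SpawnObject uses the Type value as an index into a Class array, spawns that class at the given transform, then adds the new actor to the pool retrieved from the Game Instance.
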(event `self.ReceiveBeginPlay`
  (message `/Game/Scripts/BPI_InitGM.InitFactory` (`GameplayStatics.GetGameInstance`) self)
  (`KismetSystemLibrary.PrintString` "init hecho"))

(fn `SpawnObject`
  (params (transform :type "Transform Structure") (Type :type "/Game/Scripts/EProjectyleType Enum" :default "NewEnumerator0"))
  (bind _returnvalue (`|SpawnActorFromClass` (`|GetArrayItem` (`self.Class`) (`KismetMathLibrary.Conv_ByteToInt` Type)) transform "Undefined" "MultiplyWithRoot" null null))
  (bind _poolrefe (message `/Game/Scripts/BPI_GM.GetPool` (`GameplayStatics.GetGameInstance`)))
  (message `/Game/Scripts/BPI_Pool.AddObject` _poolrefe _returnvalue))

(fn `UserConstructionScript`)